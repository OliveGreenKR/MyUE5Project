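; Player controller Blueprint for ArenaBattle that owns the player's score HUD and game result screen.
; On BeginPlay it adds the HUD to the viewport, seeds its score widget with the clear score from ABGameMode, and creates the result widget without showing it.
; Score change events update the score widget.
; Game clear and game over events set the win or loss result, then display the result widget.
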(event `self.ReceiveBeginPlay`
  (bind _returnvalue (`GameplayStatics.GetPlayerController` 0))
  ;[1 1 1] Add ABHUD to ViewPort
  (bind _returnvalue_2 (`|CreateWidget` "/Game/ArenaBattle/UI/WBP_ABHUD.WBP_ABHUD_C" _returnvalue))
  (`UserWidget.AddToViewport` _returnvalue_2 0)
  ;[1 1 1] Set PlayerScore Widget
  (bind _output_get (set `self.PlayerScoreWidger` (`/Game/ArenaBattle/UI/WBP_ABHUD.WBP_PlayerScore` _returnvalue_2)))
  (bind _clearscore (`self.GetClearScoreFromGameMode`))
  (`/Game/ArenaBattle/UI/WBP_PlayerScore.SetClearScore` _output_get _clearscore)
  ;[1 1 1] Set GameResult Widget
  (bind _returnvalue_3 (`|CreateWidget` "/Game/ArenaBattle/UI/WBP_GameResult.WBP_GameResult_C" _returnvalue))
  (set `self.GameResultWidget` _returnvalue_3))

(event `self.K2_OnScoreChanged`
  (params (NewScore :type Integer))
  ;[1 1 1] Update Score
  (`/Game/ArenaBattle/UI/WBP_PlayerScore.SetScore` (`self.PlayerScoreWidger`) NewScore))

(event `self.K2_OnGameClear`
  (bind _gameresultwidget (`self.GameResultWidget`))
  (`/Game/ArenaBattle/UI/WBP_GameResult.SetResult` _gameresultwidget true)
  (`UserWidget.AddToViewport` _gameresultwidget 0 :!label _label))

(event `self.K2_OnGameOver`
  (`/Game/ArenaBattle/UI/WBP_GameResult.SetResult` (`self.GameResultWidget`) false)
  (goto _label))

(fn `UserConstructionScript`)